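; PushySpin_BP is a VR hand-turned wheel or lever that flags when it has been rotated to a target angle.
; While its handle is overlapped and the MotionControllerPawn is grabbing, Tick pitches the whole actor along the look-at from Wheel to the right hand.
; Reaching the target pitch range sets Isdone and prints pitch for debugging.
; Ending overlap snaps rotation back to a fixed orientation, and Isdone clears while unhovered.
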(event `self.handleboi.OnComponentBeginOverlap`
  (params (OverlappedComponent :type "PrimitiveComponent Object Reference") (OtherActor :type "Actor Object Reference") (OtherComp :type "PrimitiveComponent Object Reference") (OtherBodyIndex :type Integer) (bFromSweep :type Boolean) (SweepResult :type "HitResult Structure (by ref)"))
  (set `self.IsHover` true)
  (cast `/Game/VirtualRealityBP/Blueprints/MotionControllerPawn` OtherActor))

(event `self.handleboi.OnComponentEndOverlap`
  (params (OverlappedComponent :type "PrimitiveComponent Object Reference") (OtherActor :type "Actor Object Reference") (OtherComp :type "PrimitiveComponent Object Reference") (OtherBodyIndex :type Integer))
  (set `self.IsHover` false)
  (`self.K2_SetActorRotation` (struct :`Yaw` 180.0))
  (cast `/Game/VirtualRealityBP/Blueprints/MotionControllerPawn` OtherActor))

(event `self.ReceiveTick`
  (params (DeltaSeconds :type "Float (single-precision)"))
  (bind (_returnvalue_roll _returnvalue_pitch _returnvalue_yaw) (`KismetMathLibrary.BreakRotator` (`self.K2_GetActorRotation`)))
  (bind (_returnvalue_roll_2 _returnvalue_pitch_2) (`KismetMathLibrary.BreakRotator` (`self.K2_GetActorRotation`)))
  (if (`self.IsHover`)
    (bind _asmotion_controller_pawn (cast `/Game/VirtualRealityBP/Blueprints/MotionControllerPawn` (`GameplayStatics.GetPlayerPawn` 0)))
    (if (`/Game/VirtualRealityBP/Blueprints/MotionControllerPawn.isgrabbed` _asmotion_controller_pawn)
      (bind (_returnvalue_roll_3 _returnvalue_pitch_3) (`KismetMathLibrary.BreakRotator` (`KismetMathLibrary.FindLookAtRotation` (`SceneComponent.K2_GetComponentLocation` (`self.Wheel`)) (`SceneComponent.K2_GetComponentLocation` (`/Game/VirtualRealityBP/Blueprints/BP_MotionController.HandMesh` (`/Game/VirtualRealityBP/Blueprints/MotionControllerPawn.RightController` _asmotion_controller_pawn))))))
      (`self.K2_SetActorRotation` (`KismetMathLibrary.MakeRotator` _returnvalue_roll _returnvalue_pitch_3 _returnvalue_yaw))
      (`KismetSystemLibrary.PrintString` (`KismetStringLibrary.Conv_DoubleToString` _returnvalue_pitch_2))
      (bind _output_get (set `self.hasrotated` (`KismetMathLibrary.InRange_FloatFloat` _returnvalue_pitch_2 35.0 45.0)))
      (if _output_get
        (set `self.isdone` true)))
    (else
      (set `self.isdone` false))))

(fn `UserConstructionScript`)