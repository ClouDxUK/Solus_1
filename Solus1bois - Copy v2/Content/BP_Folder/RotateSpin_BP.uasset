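; RotateSpin_BP is a VR interactable that the player turns by twisting the right motion controller.
; While something overlaps the mesh and the MotionControllerPawn is grabbing, Tick maps negated hand roll onto mesh pitch.
; Reaching a target pitch window sets Isrotated and plays an alert sound once.
; Ending overlap restores the starting rotation, and Tick then clears the flags; older HMDLocomotionPawn logic is left unwired.
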(event `self.ReceiveBeginPlay`
  (set `self.handRot` (`SceneComponent.K2_GetComponentRotation` (`self.StaticMesh`))))

(event `self.StaticMesh.OnComponentBeginOverlap`
  (params (OverlappedComponent :type "PrimitiveComponent Object Reference") (OtherActor :type "Actor Object Reference") (OtherComp :type "PrimitiveComponent Object Reference") (OtherBodyIndex :type Integer) (bFromSweep :type Boolean) (SweepResult :type "HitResult Structure (by ref)"))
  (set `self.ishover` true)
  (cast `/Game/VirtualRealityBP/Blueprints/MotionControllerPawn` OtherActor))

(event `self.StaticMesh.OnComponentEndOverlap`
  (params (OverlappedComponent :type "PrimitiveComponent Object Reference") (OtherActor :type "Actor Object Reference") (OtherComp :type "PrimitiveComponent Object Reference") (OtherBodyIndex :type Integer))
  (set `self.ishover` false)
  (`SceneComponent.K2_SetWorldRotation` (`self.StaticMesh`) (`self.handRot`) false false)
  (cast `/Game/VirtualRealityBP/Blueprints/MotionControllerPawn` OtherActor))

(event `self.ReceiveTick`
  (params (DeltaSeconds :type "Float (single-precision)"))
  (bind _staticmesh (`self.StaticMesh`))
  (bind (_returnvalue_roll _returnvalue_pitch) (`KismetMathLibrary.BreakRotator` (`SceneComponent.K2_GetComponentRotation` _staticmesh)))
  (if (`self.ishover`)
    (bind _asmotion_controller_pawn (cast `/Game/VirtualRealityBP/Blueprints/MotionControllerPawn` (`GameplayStatics.GetPlayerPawn` 0)))
    (if (`/Game/VirtualRealityBP/Blueprints/MotionControllerPawn.isgrabbed` _asmotion_controller_pawn)
      (bind _returnvalue_roll_2 (`KismetMathLibrary.BreakRotator` (`SceneComponent.K2_GetComponentRotation` (`/Game/VirtualRealityBP/Blueprints/BP_MotionController.HandMesh` (`/Game/VirtualRealityBP/Blueprints/MotionControllerPawn.RightController` _asmotion_controller_pawn)))))
      (`SceneComponent.K2_SetRelativeRotation` _staticmesh (`KismetMathLibrary.MakeRotator` 0.0 (* _returnvalue_roll_2 -1.0)) false false)
      (`SceneComponent.K2_SetRelativeRotation` (`self.StaticMeshComponent`) (`KismetMathLibrary.MakeRotator` 0.0 (* _returnvalue_roll_2 -1.0)) false false)
      (`KismetSystemLibrary.PrintString` (`KismetStringLibrary.Conv_DoubleToString` _returnvalue_pitch))
      (bind _output_get (set `self.madeonce` (`KismetMathLibrary.InRange_FloatFloat` _returnvalue_pitch 40.0 50.0)))
      (if _output_get
        (set `self.isrotated` true)
        (if (not (`self.played audio`))
          (set `self.played audio` true)
          (`GameplayStatics.PlaySoundAtLocation` "/Game/Metal_Gear_Alert_Sound_Effect.Metal_Gear_Alert_Sound_Effect" (`SceneComponent.K2_GetComponentLocation` (`self.StaticMesh`)) (struct) 1.0 1.0 0.0 null null null))))
    (else
      (set `self.isrotated` false)
      (set `self.madeonce` false)
      (set `self.played audio` false))))

(fn `UserConstructionScript`)