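; PushSpin_BP is an actor that the VR player can rotate by grabbing it.
; Overlap events on its static mesh set a hover flag while an HMDLocomotionPawn is in contact.
; Each tick, if hovered and the player pawn reports a grab, the actor copies the world rotation of the pawn's Sausage component directly, with no offset.
; The mesh's starting rotation is stored at BeginPlay but never used.
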(event `self.ReceiveBeginPlay`
  (set `self.StartRot` (`SceneComponent.K2_GetComponentRotation` (`self.StaticMeshComponent`))))

(event `self.StaticMeshComponent.OnComponentBeginOverlap`
  (params (OverlappedComponent :type "PrimitiveComponent Object Reference") (OtherActor :type "Actor Object Reference") (OtherComp :type "PrimitiveComponent Object Reference") (OtherBodyIndex :type Integer) (bFromSweep :type Boolean) (SweepResult :type "HitResult Structure (by ref)"))
  (cast `/Game/VirtualRealityBP/Blueprints/HMDLocomotionPawn` OtherActor)
  (set `self.ishover` true))

(event `self.StaticMeshComponent.OnComponentEndOverlap`
  (params (OverlappedComponent :type "PrimitiveComponent Object Reference") (OtherActor :type "Actor Object Reference") (OtherComp :type "PrimitiveComponent Object Reference") (OtherBodyIndex :type Integer))
  (cast `/Game/VirtualRealityBP/Blueprints/HMDLocomotionPawn` OtherActor)
  (set `self.ishover` false))

(event `self.ReceiveTick`
  (params (DeltaSeconds :type "Float (single-precision)"))
  (if (`self.ishover`)
    (bind _ashmdlocomotion_pawn (cast `/Game/VirtualRealityBP/Blueprints/HMDLocomotionPawn` (`GameplayStatics.GetPlayerPawn` 0)))
    (if (`/Game/VirtualRealityBP/Blueprints/HMDLocomotionPawn.IsGrabbed` _ashmdlocomotion_pawn)
      (`self.K2_SetActorRotation` (`SceneComponent.K2_GetComponentRotation` (`/Game/VirtualRealityBP/Blueprints/HMDLocomotionPawn.sausage` _ashmdlocomotion_pawn))))))

(fn `UserConstructionScript`)