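; VR puzzle piece: a small pyramid the player turns by grabbing, driving the yaw of BigPyra4.
; Each tick, while overlapped and grabbed, it yaws toward the right hand, with roll and pitch oddly fed from actor location.
; Yaw near zero latches it in place, stops the mirroring, snaps the mesh to a fixed rotation and plays an alert sound once.
; Hover is set by any overlap, before the pawn cast.
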(event `self.ReceiveTick`
  (params (DeltaSeconds :type "Float (single-precision)"))
  (bind _staticmeshcomponent (`self.StaticMeshComponent`))
  (bind (_returnvalue_roll _returnvalue_pitch _returnvalue_yaw) (`KismetMathLibrary.BreakRotator` (`SceneComponent.K2_GetComponentRotation` (`self.StaticMeshComponent`))))
  (`self.InputRot`)
  (if (`self.isinplace`)
    (set `self.isinplace` true)
    (if (not (`self.completed`))
      (set `self.completed` true)
      (`SceneComponent.K2_SetWorldRotation` _staticmeshcomponent (struct :`Yaw` 180.0) false false)
      (`GameplayStatics.PlaySoundAtLocation` "/Game/Metal_Gear_Alert_Sound_Effect.Metal_Gear_Alert_Sound_Effect" (`SceneComponent.K2_GetComponentLocation` _staticmeshcomponent) (struct) 0.5 1.0 0.0 null null null))
    (else
      (set `self.isinplace` (`KismetMathLibrary.InRange_FloatFloat` _returnvalue_yaw -1.0 1.0))
      (`SceneComponent.K2_SetWorldRotation` (`Actor.RootComponent` (`self.BigPyra4`)) (`KismetMathLibrary.MakeRotator` 0.0 0.0 _returnvalue_yaw) false false))))

(event `InputRot`
  (bind (_returnvalue_x _returnvalue_y) (`KismetMathLibrary.BreakVector` (`self.K2_GetActorLocation`)))
  (if (`self.ishover`)
    (bind _asmotion_controller_pawn (cast `/Game/VirtualRealityBP/Blueprints/MotionControllerPawn` (`GameplayStatics.GetPlayerPawn` 0)))
    (if (`/Game/VirtualRealityBP/Blueprints/MotionControllerPawn.isgrabbed` _asmotion_controller_pawn)
      (bind (_returnvalue_roll _returnvalue_pitch _returnvalue_yaw) (`KismetMathLibrary.BreakRotator` (`KismetMathLibrary.FindLookAtRotation` (`SceneComponent.K2_GetComponentLocation` (`self.StaticMeshComponent`)) (`SceneComponent.K2_GetComponentLocation` (`/Game/VirtualRealityBP/Blueprints/BP_MotionController.HandMesh` (`/Game/VirtualRealityBP/Blueprints/MotionControllerPawn.RightController` _asmotion_controller_pawn))))))
      (`self.K2_SetActorRotation` (`KismetMathLibrary.MakeRotator` _returnvalue_x _returnvalue_y _returnvalue_yaw)))))

(event `self.StaticMeshComponent.OnComponentBeginOverlap`
  (params (OverlappedComponent :type "PrimitiveComponent Object Reference") (OtherActor :type "Actor Object Reference") (OtherComp :type "PrimitiveComponent Object Reference") (OtherBodyIndex :type Integer) (bFromSweep :type Boolean) (SweepResult :type "HitResult Structure (by ref)"))
  (set `self.ishover` true)
  (cast `/Game/VirtualRealityBP/Blueprints/MotionControllerPawn` OtherActor))

(event `self.StaticMeshComponent.OnComponentEndOverlap`
  (params (OverlappedComponent :type "PrimitiveComponent Object Reference") (OtherActor :type "Actor Object Reference") (OtherComp :type "PrimitiveComponent Object Reference") (OtherBodyIndex :type Integer))
  (set `self.ishover` false)
  (cast `/Game/VirtualRealityBP/Blueprints/MotionControllerPawn` OtherActor))

(fn `UserConstructionScript`)