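; A pullable sphere for VR that follows the player's right hand while grabbed, trailed by three rings.
; Any overlap sets a hover flag; while hovered, Tick moves the actor to the MotionControllerPawn's hand if grabbed, otherwise back to its BeginPlay location.
; VInterpTo with a constant DeltaTime acts as a fixed blend, spacing the rings between start and current positions and making the return an instant snap.
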(event `self.ReceiveBeginPlay`
  (set `self.startloc` (`SceneComponent.K2_GetComponentLocation` (`self.StaticMeshComponent`))))

(event `self.Sphere.OnComponentBeginOverlap`
  (params (OverlappedComponent :type "PrimitiveComponent Object Reference") (OtherActor :type "Actor Object Reference") (OtherComp :type "PrimitiveComponent Object Reference") (OtherBodyIndex :type Integer) (bFromSweep :type Boolean) (SweepResult :type "HitResult Structure (by ref)"))
  (set `self.ishover` true)
  (cast `/Game/VirtualRealityBP/Blueprints/MotionControllerPawn` OtherActor))

(event `self.Sphere.OnComponentEndOverlap`
  (params (OverlappedComponent :type "PrimitiveComponent Object Reference") (OtherActor :type "Actor Object Reference") (OtherComp :type "PrimitiveComponent Object Reference") (OtherBodyIndex :type Integer))
  (set `self.ishover` false)
  (cast `/Game/VirtualRealityBP/Blueprints/MotionControllerPawn` OtherActor))

(event `self.ReceiveTick`
  (params (DeltaSeconds :type "Float (single-precision)"))
  (set `self.isdone` false)
  (`self.K2_SetActorLocation` (`self.Ring1`) (`KismetMathLibrary.VInterpTo` (`self.startloc`) (`SceneComponent.K2_GetComponentLocation` (`self.StaticMeshComponent`)) 1.0 0.7) false false)
  (`self.K2_SetActorLocation` (`self.Ring2`) (`KismetMathLibrary.VInterpTo` (`self.startloc`) (`SceneComponent.K2_GetComponentLocation` (`self.StaticMeshComponent`)) 1.0 0.5) false false)
  (`self.K2_SetActorLocation` (`self.Ring3`) (`KismetMathLibrary.VInterpTo` (`self.startloc`) (`SceneComponent.K2_GetComponentLocation` (`self.StaticMeshComponent`)) 1.0 0.3) false false)
  (if (`self.ishover`)
    (bind _asmotion_controller_pawn (cast `/Game/VirtualRealityBP/Blueprints/MotionControllerPawn` (`GameplayStatics.GetPlayerPawn` 0)))
    (if (`/Game/VirtualRealityBP/Blueprints/MotionControllerPawn.isgrabbed` _asmotion_controller_pawn)
      (`self.K2_SetActorLocation` (`SceneComponent.K2_GetComponentLocation` (`/Game/VirtualRealityBP/Blueprints/BP_MotionController.HandMesh` (`/Game/VirtualRealityBP/Blueprints/MotionControllerPawn.RightController` _asmotion_controller_pawn))))
      (else
        (`self.returnLoc`)))))

(event `returnLoc`
  (`self.K2_SetActorLocation` (`KismetMathLibrary.VInterpTo` (`SceneComponent.K2_GetComponentLocation` (`self.StaticMeshComponent`)) (`self.startloc`) 1.0 1.0))
  (set `self.isdone` false))

(fn `UserConstructionScript`)