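; VR door Blueprint that swings to follow the player's right hand while its handle is overlapped.
; Overlap events on the handle toggle a hover flag before casting to MotionControllerPawn, so any overlapping actor sets it.
; While hovered, Tick aims the mesh at the right controller's hand using only look-at pitch, zeroing world roll and yaw.
; BeginPlay stores the starting rotation, which the graph never uses.
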(event `self.ReceiveBeginPlay`
  (bind (_returnvalue_roll _returnvalue_pitch _returnvalue_yaw) (`KismetMathLibrary.BreakRotator` (`SceneComponent.K2_GetComponentRotation` (`self.StaticMeshComponent`))))
  (set `self.startRot` (`KismetMathLibrary.MakeVector` _returnvalue_roll _returnvalue_pitch _returnvalue_yaw)))

(event `self.handledoor.OnComponentBeginOverlap`
  (params (OverlappedComponent :type "PrimitiveComponent Object Reference") (OtherActor :type "Actor Object Reference") (OtherComp :type "PrimitiveComponent Object Reference") (OtherBodyIndex :type Integer) (bFromSweep :type Boolean) (SweepResult :type "HitResult Structure (by ref)"))
  (set `self.ishover` true)
  (cast `/Game/VirtualRealityBP/Blueprints/MotionControllerPawn` OtherActor))

(event `self.handledoor.OnComponentEndOverlap`
  (params (OverlappedComponent :type "PrimitiveComponent Object Reference") (OtherActor :type "Actor Object Reference") (OtherComp :type "PrimitiveComponent Object Reference") (OtherBodyIndex :type Integer))
  (set `self.ishover` false)
  (cast `/Game/VirtualRealityBP/Blueprints/MotionControllerPawn` OtherActor))

(event `self.ReceiveTick`
  (params (DeltaSeconds :type "Float (single-precision)"))
  (bind _staticmeshcomponent (`self.StaticMeshComponent`))
  (if (`self.ishover`)
    (bind _asmotion_controller_pawn (cast `/Game/VirtualRealityBP/Blueprints/MotionControllerPawn` (`GameplayStatics.GetPlayerPawn` 0)))
    (bind (_returnvalue_roll _returnvalue_pitch) (`KismetMathLibrary.BreakRotator` (`KismetMathLibrary.FindLookAtRotation` (`SceneComponent.K2_GetComponentLocation` _staticmeshcomponent) (`SceneComponent.K2_GetComponentLocation` (`/Game/VirtualRealityBP/Blueprints/BP_MotionController.HandMesh` (`/Game/VirtualRealityBP/Blueprints/MotionControllerPawn.RightController` _asmotion_controller_pawn))))))
    (`SceneComponent.K2_SetWorldRotation` _staticmeshcomponent (`KismetMathLibrary.MakeRotator` 0.0 _returnvalue_pitch) false false)))

(fn `UserConstructionScript`)