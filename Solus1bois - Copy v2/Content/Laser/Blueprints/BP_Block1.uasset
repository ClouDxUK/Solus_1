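; BP_Block1 is a laser emitter that fires a beam from its Arrow and reflects it off surfaces using M_Mirror.
; Each Tick loops up to MaxBounces, line tracing from stored hit points and mirroring the direction by the impact normal.
; Every segment spawns a coloured PS_Beam emitter, then the arrays clear and reseed from the Arrow.
; An unconnected branch would change a BP_Endpoint's material after enough bounces.
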(event `self.ReceiveTick`
  (params (DeltaSeconds :type "Float (single-precision)"))
  (bind _arrow (`self.Arrow`))
  (bind _hit_location (`self.Hit Location`))
  (bind _output (`|GetArrayItem` (`self.Hit Location`) (`self.Current Index`)))
  (bind _output_2 (`|GetArrayItem` (`self.Hit Location`) (`self.Current Index`)))
  ;[1 1 1] Debug
  ;[1 1 1] Looper
  (for _index (range (+ (`self.Max Bounces`) 1))
    ;[1 1 1] Counts how many bounces the laser has made
    (set `self.Current Index` _index)
    (set `self.Current Bounce` 0)
    (for _array_element (`self.Bounce True`)
      (if _array_element
        (`/Engine/EditorBlueprintResources/StandardMacros.IncrementInt` (`self.Current Bounce`))))
    ;[1 1 1] Laser Generation & Hit Detection
    (bind (_outhit _returnvalue) (`KismetSystemLibrary.LineTraceSingleForObjects` _output_2 (+ _output_2 (* (`|GetArrayItem` (`self.Laser Direction`) (`self.Current Index`)) (`self.Laser Length`))) (`|MakeArray` "ObjectTypeQuery1" "ObjectTypeQuery2" "ObjectTypeQuery4" :!type "EObjectTypeQuery Enum") true))
    (if _returnvalue
      (bind (_bblockinghit _binitialoverlap _time _distance _location _impactpoint _normal _impactnormal _physmat _hitactor _hitcomponent) (`GameplayStatics.BreakHitResult` _outhit))
      (set `self.Laser Hit Location` _impactpoint)
      (set `self.Laser Normal` (`KismetMathLibrary.MirrorVectorByNormal` (`|GetArrayItem` (`self.Laser Direction`) (`self.Current Index`)) _impactnormal))
      (set `self.Reflective Material` (== (`PrimitiveComponent.GetMaterial` _hitcomponent 0) "/Game/Laser/M_Mirror.M_Mirror"))
      (if (`self.Reflective Material`)
        (`KismetArrayLibrary.Array_Add` (`self.Hit Location`) (`self.Laser Hit Location`))
        (`KismetArrayLibrary.Array_Add` (`self.Laser Direction`) (`self.Laser Normal`))
        (`KismetArrayLibrary.Array_Add` (`self.Bounce True`) true)
        (bind _returnvalue_2 (`GameplayStatics.SpawnEmitterAtLocation` "/Game/Laser/ParticleSystem/PS_Beam.PS_Beam" (`|GetArrayItem` _hit_location (`self.Current Index`))))
        (`ParticleSystemComponent.SetBeamTargetPoint` _returnvalue_2 0 (`|GetArrayItem` _hit_location (+ (`self.Current Index`) 1)) 0)
        (`ParticleSystemComponent.SetColorParameter` _returnvalue_2 "Colour" (`self.Beam Colour`))
        (else
          (`KismetArrayLibrary.Array_Add` (`self.Bounce True`))
          (bind _returnvalue_3 (`GameplayStatics.SpawnEmitterAtLocation` "/Game/Laser/ParticleSystem/PS_Beam.PS_Beam" (`|GetArrayItem` (`self.Hit Location`) (`self.Current Index`))))
          (`ParticleSystemComponent.SetBeamTargetPoint` _returnvalue_3 0 (`self.Laser Hit Location`) 0)
          (`ParticleSystemComponent.SetColorParameter` _returnvalue_3 "Colour" (`self.Beam Colour`))))
      (else
        (`KismetArrayLibrary.Array_Add` (`self.Bounce True`))
        (bind _returnvalue_4 (`GameplayStatics.SpawnEmitterAtLocation` "/Game/Laser/ParticleSystem/PS_Beam.PS_Beam" _output))
        (`ParticleSystemComponent.SetBeamTargetPoint` _returnvalue_4 0 (+ _output (* (`|GetArrayItem` (`self.Laser Direction`) (`self.Current Index`)) (`self.Laser Length`))) 0)
        (`ParticleSystemComponent.SetColorParameter` _returnvalue_4 "Colour" (`self.Beam Colour`)))))
  ;[1 1 1] Clean up
  (`KismetArrayLibrary.Array_Clear` (`self.Hit Location`))
  (`KismetArrayLibrary.Array_Clear` (`self.Laser Direction`))
  (`KismetArrayLibrary.Array_Clear` (`self.Bounce True`))
  ;[1 1 1] Root
  (`KismetArrayLibrary.Array_Add` (`self.Hit Location`) (`SceneComponent.K2_GetComponentLocation` _arrow) :!label _label)
  (`KismetArrayLibrary.Array_Add` (`self.Laser Direction`) (`SceneComponent.GetForwardVector` _arrow)))

(event `self.ReceiveBeginPlay`
  ;[1 1 1] Root
  (goto _label))

(fn `UserConstructionScript`)