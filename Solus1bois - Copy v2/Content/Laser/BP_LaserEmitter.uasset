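; BP_LaserEmitter is a laser emitter actor that traces a light path from its Arrow, reflecting off mirror surfaces.
; Tick, through a short Delay, calls CastLight, which destroys old beams and loops line traces.
; Hits on M_Mirror faces, identified by collision face material, reflect the direction about the impact normal; anything else ends the loop.
; Beam spawning is disconnected, so only persistent debug traces show the path.
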(event `self.ReceiveTick`
  (params (DeltaSeconds :type "Float (single-precision)"))
  (bind _arrow (`self.Arrow`))
  (`KismetSystemLibrary.Delay` 0.01)
  (`self.Cast_Light` (`SceneComponent.K2_GetComponentLocation` _arrow) (`SceneComponent.GetForwardVector` _arrow) (`self.Cast Distance`)))

(fn `Cast_Light`
  (params (CastOrigin :type "Vector Structure") (CastDirection :type "Vector Structure") (CastDistance :type "Float (double-precision)"))
  (locals (L_CastOrigin :type "Vector Structure") (L_CastDirection :type "Vector Structure") (L_CastDistance :type "Float (double-precision)") (L_Continue :type Boolean :default true) (L_Beamstart :type "Vector Structure") (L_BeamEnd :type "Vector Structure") (NewLocalVar_0 :type "Array of String"))
  (bind _l_castorigin (`local.L_CastOrigin`))
  (set `local.L_CastOrigin` CastOrigin)
  (set `local.L_CastDirection` CastDirection)
  (set `local.L_CastDistance` CastDistance)
  (for _array_element (`self.Beams`)
    (`self.K2_DestroyActor` _array_element))
  (`KismetArrayLibrary.Array_Clear` (`self.Beams`))
  (while (`local.L_Continue`)
    (`|ExecutionSequence`
      (:`then_0`
        (bind (_outhit _returnvalue) (`KismetSystemLibrary.LineTraceSingle` :`Start` _l_castorigin :`End` (+ _l_castorigin (* (`local.L_CastDirection`) (`local.L_CastDistance`))) :`TraceChannel` "TraceTypeQuery1" :`bTraceComplex` true :`DrawDebugType` "Persistent"))
        (set `local.L_Beamstart` (`local.L_CastOrigin`))
        (if _returnvalue
          (bind (_bblockinghit _binitialoverlap _time _distance _location _impactpoint _normal _impactnormal _physmat _hitactor _hitcomponent _hitbonename _hititem _faceindex) (`GameplayStatics.BreakHitResult` _outhit))
          (set `local.L_BeamEnd` _impactpoint)
          (if (== (`.ReturnValue` (`PrimitiveComponent.GetMaterialFromCollisionFaceIndex` _hitcomponent _faceindex)) "/Game/Laser/M_Mirror.M_Mirror")
            (set `local.L_CastOrigin` _impactpoint)
            (set `local.L_CastDirection` (`KismetMathLibrary.MirrorVectorByNormal` (`local.L_CastDirection`) _impactnormal))
            (set `local.L_Continue` true)
            (else
              (set `local.L_BeamEnd` _impactpoint :!label _label)
              (set `local.L_Continue` false)))
          (else
            (goto _label))))
      (:`then_2`
        (while false
          _)))))

(fn `UserConstructionScript`)